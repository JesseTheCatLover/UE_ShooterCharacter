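; Grux enemy character Blueprint that drives the UI for its health bar and floating hit numbers.
; On BeginPlay it binds itself to the health bar widget, which show and hide events toggle, with showing also calling the parent implementation.
; Each hit spawns a HitNumber widget at the projected screen position, registers it with its world location via StoreHitNumber, then sets damage text and headshot flag and plays its animation.
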(event EventBeginPlay
  (bind _asenemy_heatlh_bar (Utilities|Casting|CastToEnemyHeatlhBar (UserInterface|GetWidget (Variables|Default|GetHealthBar))))
  (Variables|/Game/_Game/HUD/EnemyHeatlhBar.EnemyHeatlhBar_C|SetEnemy _asenemy_heatlh_bar self))

(event Collision|EventActorBeginOverlap
  (params (OtherActor :type Actor%20Object%20Reference)))

(event EventTick
  (params (DeltaSeconds :type Float%20%28single-precision%29)))

(event EventShowHealthBar
  (Widget|SetVisibility (UserInterface|GetWidget (Variables|Default|GetHealthBar)) "Visible")
  (|CallParentFunction))

(event EventHideHealthBar
  (Widget|SetVisibility (UserInterface|GetWidget (Variables|Default|GetHealthBar)) "Hidden"))

(event EventShowHitNumber
  (params (Damage :type Integer) (HitLocation :type Vector :default "0, 0, 0") (bHeadShot :type Boolean))
  (bind _returnvalue (UserInterface|CreateWidget "/Game/_Game/HUD/HitNumber.HitNumber_C"))
  (UserInterface|Viewport|AddtoViewport _returnvalue 0)
  (Class|UserWidget|SetPositioninViewport _returnvalue (.ScreenLocation (Class|PlayerController|ProjectWorldLocationtoScreen (Game|GetPlayerController 0) HitLocation false)) true)
  (Class|Enemy|StoreHitNumber _returnvalue HitLocation)
  (Variables|/Game/_Game/HUD/HitNumber.HitNumber_C|SetHitText _returnvalue (Utilities|Text|ToText(Integer) Damage))
  (Variables|/Game/_Game/HUD/HitNumber.HitNumber_C|SetHeadShot _returnvalue bHeadShot)
  (UserInterface|Animation|PlayAnimation _returnvalue (Variables|/Game/_Game/HUD/HitNumber.HitNumber_C|GetHitNumberAnim _returnvalue) 0.0 1 "Forward" 1.0 false))

(fn ConstructionScript)